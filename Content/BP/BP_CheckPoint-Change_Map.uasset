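; Trigger-box actor that works as either a checkpoint or a map-change point, selected by the ECheckPointOrChangeMap enum.
; On overlap, checkpoint mode saves the BP_ThirdPersonCharacter's capsule position as its RespawnLocation.
; Change-map mode, without checking the overlapping actor, creates WBP_Main on its second switcher page and shows the mouse cursor; no level loads here.
; The mesh location stored at BeginPlay is unused in these graphs.
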(event OnComponentBeginOverlap(Box)
  (params (OverlappedComponent :type Primitive%20Component%20Object%20Reference) (OtherActor :type Actor%20Object%20Reference) (OtherComp :type Primitive%20Component%20Object%20Reference) (OtherBodyIndex :type Integer) (bFromSweep :type Boolean) (SweepResult :type Hit%20Result%20Structure%20%28by%20ref%29))
  (bind _output_get (Variables|Default|SetCan_Respawn? true))
  (if _output_get
    (switch Utilities|FlowControl|Switch|SwitchonE_CheckPoint_or_ChangeMap (Variables|Default|Get%20E_CheckPoint_or_ChangeMap)
      (:NewEnumerator0
        (Variables|Default|SetTo_Respawn true)
        (bind _asbp_third_person_character (Utilities|Casting|CastToBP_ThirdPersonCharacter OtherActor))
        (Variables|/Game/ThirdPerson/Blueprints/BP_ThirdPersonCharacter.BP_ThirdPersonCharacter_C|SetRespawn_Location _asbp_third_person_character (Transformation|GetWorldLocation (Variables|/Script/Engine.Character|GetCapsuleComponent _asbp_third_person_character))))
      (:NewEnumerator1
        (Variables|Default|SetTo_ChangeMap true)
        (bind _returnvalue (UserInterface|CreateWidget "/Game/Widget/WBP_Main.WBP_Main_C"))
        (Variables|/Script/UMG.WidgetSwitcher|SetActiveWidgetIndex (Variables|/Game/Widget/WBP_Main.WBP_Main_C|GetWidgetSwitcher _returnvalue) 1)
        (Variables|/Script/Engine.PlayerController|SetbShowMouseCursor (Variables|/Game/Widget/WBP_Main.WBP_Main_C|GetControlerRef _returnvalue) true)
        (UserInterface|Viewport|AddtoViewport _returnvalue 0)))))

(event EventBeginPlay
  (Variables|Default|SetCan_Respawn? false)
  (Variables|Default|SetRespawn_At_CheckPoint (Transformation|GetWorldLocation (Variables|Default|GetStaticMesh)))
  (Variables|Default|SetTo_Respawn false)
  (Variables|Default|SetTo_ChangeMap false))

(fn ConstructionScript)